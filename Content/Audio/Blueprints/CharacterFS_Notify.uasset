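; Footstep anim notify that plays surface-specific sounds at the left or right foot socket.
; It matches player character 0's floor surface against SurfaceTypes to choose one of eight sound arrays, then randomizes pick, volume and pitch.
; Landings play louder from the array's tail, while steps use index bounds from the character's DetermineRandomBounds.
; SelectFSBasedOnSpeed, a walk/jog/run picker by normalized speed, is not called by the notify.
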(fn ReceivedNotify
  (params (MeshComp :type Skeletal%20Mesh%20Component%20Object%20Reference) (Animation :type Anim%20Sequence%20Base%20Object%20Reference))
  (if (Variables|Default|GetisLeftFoot)
    (LocalVariables|SetSocketName "FSSoundSocket_L")
    (else
      (LocalVariables|SetSocketName "FSSoundSocket_R")))
  (bind _asthird_person_character (Utilities|Casting|CastToThirdPersonCharacter (Game|GetPlayerCharacter 0)))
  (for (_array_element _array_index) (Variables|Default|GetSurfaceTypes)
    (if (Utilities|Enum|Equal(Enum) _array_element (Utilities|GetDisplayName (Variables|/Game/Assets_Character/Protaganist/ThirdPersonCharacter.ThirdPersonCharacter_C|GetFloorSurfaceType _asthird_person_character)))
      (if (Variables|Default|GetisLanding)
        (Audio|PlaySoundatLocation (Utilities|Array|Get(acopy) (Utilities|Select :Index (Math|Integer|Clamp(Integer) (- _array_index 1) 0 7) :Option%200 (Variables|Default|GetFS_SandDry) :Option%201 (Variables|Default|GetFS_SandWet) :Option%202 (Variables|Default|GetFS_Concrete) :Option%203 (Variables|Default|GetFS_Metal) :Option%204 (Variables|Default|GetFS_WaterShallow) :Option%205 (Variables|Default|GetFS_WaterDeep) :Option%206 (Variables|Default|GetFS_Wood) :Option%207 (Variables|Default|GetFS_Glass)) (Math|Random|RandomIntegerinRange (- (Utilities|Array|Length (Utilities|Select :Index (Math|Integer|Clamp(Integer) (- _array_index 1) 0 7) :Option%200 (Variables|Default|GetFS_SandDry) :Option%201 (Variables|Default|GetFS_SandWet) :Option%202 (Variables|Default|GetFS_Concrete) :Option%203 (Variables|Default|GetFS_Metal) :Option%204 (Variables|Default|GetFS_WaterShallow) :Option%205 (Variables|Default|GetFS_WaterDeep) :Option%206 (Variables|Default|GetFS_Wood) :Option%207 (Variables|Default|GetFS_Glass))) 3) (Utilities|Array|Length (Utilities|Select :Index (Math|Integer|Clamp(Integer) (- _array_index 1) 0 7) :Option%200 (Variables|Default|GetFS_SandDry) :Option%201 (Variables|Default|GetFS_SandWet) :Option%202 (Variables|Default|GetFS_Concrete) :Option%203 (Variables|Default|GetFS_Metal) :Option%204 (Variables|Default|GetFS_WaterShallow) :Option%205 (Variables|Default|GetFS_WaterDeep) :Option%206 (Variables|Default|GetFS_Wood) :Option%207 (Variables|Default|GetFS_Glass))))) (Transformation|GetSocketLocation MeshComp (LocalVariables|GetSocketName)) "0, 0, 0" (Math|Random|RandomFloatinRange 1.45 1.65) (Math|Random|RandomFloatinRange 0.95 1.05) 0.0 "/Game/Audio/SoundAttenuations/ATT_PlayerFS.ATT_PlayerFS")
        (else
          (Audio|PlaySoundatLocation (Utilities|Array|Get(acopy) (Utilities|Select :Index (Math|Integer|Clamp(Integer) (- _array_index 1) 0 7) :Option%200 (Variables|Default|GetFS_SandDry) :Option%201 (Variables|Default|GetFS_SandWet) :Option%202 (Variables|Default|GetFS_Concrete) :Option%203 (Variables|Default|GetFS_Metal) :Option%204 (Variables|Default|GetFS_WaterShallow) :Option%205 (Variables|Default|GetFS_WaterDeep) :Option%206 (Variables|Default|GetFS_Wood) :Option%207 (Variables|Default|GetFS_Glass)) (Math|Random|RandomIntegerinRange (Math|Integer|Clamp(Integer) (.RandomLowerBound (|DetermineRandomBounds _asthird_person_character (Utilities|Select :Index (Math|Integer|Clamp(Integer) (- _array_index 1) 0 7) :Option%200 (Variables|Default|GetFS_SandDry) :Option%201 (Variables|Default|GetFS_SandWet) :Option%202 (Variables|Default|GetFS_Concrete) :Option%203 (Variables|Default|GetFS_Metal) :Option%204 (Variables|Default|GetFS_WaterShallow) :Option%205 (Variables|Default|GetFS_WaterDeep) :Option%206 (Variables|Default|GetFS_Wood) :Option%207 (Variables|Default|GetFS_Glass)))) 0 (.TargetedArrayIndex (|DetermineRandomBounds _asthird_person_character (Utilities|Select :Index (Math|Integer|Clamp(Integer) (- _array_index 1) 0 7) :Option%200 (Variables|Default|GetFS_SandDry) :Option%201 (Variables|Default|GetFS_SandWet) :Option%202 (Variables|Default|GetFS_Concrete) :Option%203 (Variables|Default|GetFS_Metal) :Option%204 (Variables|Default|GetFS_WaterShallow) :Option%205 (Variables|Default|GetFS_WaterDeep) :Option%206 (Variables|Default|GetFS_Wood) :Option%207 (Variables|Default|GetFS_Glass))))) (Math|Integer|Clamp(Integer) (.TargetedArrayLength (|DetermineRandomBounds _asthird_person_character (Utilities|Select :Index (Math|Integer|Clamp(Integer) (- _array_index 1) 0 7) :Option%200 (Variables|Default|GetFS_SandDry) :Option%201 (Variables|Default|GetFS_SandWet) :Option%202 (Variables|Default|GetFS_Concrete) :Option%203 (Variables|Default|GetFS_Metal) :Option%204 (Variables|Default|GetFS_WaterShallow) :Option%205 (Variables|Default|GetFS_WaterDeep) :Option%206 (Variables|Default|GetFS_Wood) :Option%207 (Variables|Default|GetFS_Glass)))) 0 (.TargetedArrayIndex (|DetermineRandomBounds _asthird_person_character (Utilities|Select :Index (Math|Integer|Clamp(Integer) (- _array_index 1) 0 7) :Option%200 (Variables|Default|GetFS_SandDry) :Option%201 (Variables|Default|GetFS_SandWet) :Option%202 (Variables|Default|GetFS_Concrete) :Option%203 (Variables|Default|GetFS_Metal) :Option%204 (Variables|Default|GetFS_WaterShallow) :Option%205 (Variables|Default|GetFS_WaterDeep) :Option%206 (Variables|Default|GetFS_Wood) :Option%207 (Variables|Default|GetFS_Glass))))))) (Transformation|GetSocketLocation MeshComp (LocalVariables|GetSocketName)) "0, 0, 0" (Math|Random|RandomFloatinRange 1.0 1.05) (Math|Random|RandomFloatinRange 0.95 1.05) 0.0 "/Game/Audio/SoundAttenuations/ATT_PlayerFS.ATT_PlayerFS")))
      (return false))))

(fn SelectFSBasedonSpeed
  (params (NormalizedPlayerSpeed :type Float%20%28single-precision%29) (FS_Sounds :type Array%20of%20Sound%20Wave%20Object%20References))
  (bind _returnvalue (Utilities|Array|Length FS_Sounds))
  (bind _returnvalue_2 (Math|Float|Clamp(Float) NormalizedPlayerSpeed))
  (bind _returnvalue_3 (|MaxWalk+1))
  (bind _value (|MaxJog+1))
  (bind _maxindexjogging (Variables|Default|GetMaxIndexJogging))
  (bind _returnvalue_4 (Math|Random|RandomIntegerinRange _value _returnvalue))
  (bind _returnvalue_5 (Math|Random|RandomIntegerinRange _returnvalue_3 _maxindexjogging))
  (bind _output (Utilities|Array|Get(acopy) FS_Sounds _returnvalue_4))
  (bind _output_2 (Utilities|Array|Get(acopy) FS_Sounds _returnvalue_5))
  (if (Math|Float|InRange(Float) _returnvalue_2 0.0 0.34)
    (Utilities|IsValid (Utilities|Array|Get(acopy) FS_Sounds (Math|Random|RandomIntegerinRange 0 (Variables|Default|GetMaxIndexWalking)))
      (:Is%20Valid
        (return 0))
      (:Is%20Not%20Valid
        (return (Utilities|Array|Get(acopy) FS_Sounds 1))))
    (elif (Math|Float|InRange(Float) _returnvalue_2 0.3401 0.67)
      (Utilities|IsValid _output_2
        (:Is%20Valid
          (return _output_2))
        (:Is%20Not%20Valid
          (return (Utilities|Array|Get(acopy) FS_Sounds _returnvalue_3))))
      (elif (Math|Float|InRange(Float) _returnvalue_2 0.6701 2.0)
        (Utilities|IsValid _output
          (:Is%20Valid
            (return _output))
          (:Is%20Not%20Valid
            (return (Utilities|Array|Get(acopy) FS_Sounds _value))))))))