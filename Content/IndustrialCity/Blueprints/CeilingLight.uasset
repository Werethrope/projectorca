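; CeilingLight is a placeable ceiling light fixture for the IndustrialCity content, pairing a static mesh with a spotlight.
; The construction script creates a dynamic material instance on the mesh and applies the shadow and intensity settings to the spotlight.
; LightToggle switches spotlight visibility and writes a material scalar, though its parameter name is None and both branches evaluate to zero for nonzero intensity.
; The event graph has no runtime logic.
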(event EventBeginPlay)

(event EventActorBeginOverlap
  (params (OtherActor :type Actor%20Object%20Reference)))

(event EventTick
  (params (DeltaSeconds :type Float%20%28single-precision%29)))

(fn ConstructionScript
  (bind _spotlight (Variables|Default|GetSpotLight))
  (bind _lightintensity (Variables|Default|GetLightIntensity))
  (bind _returnvalue (Rendering|Material|CreateDynamicMaterialInstance (Variables|Default|GetStaticMesh) 0 "/Game/IndustrialCity/Materials/CeilingLight.CeilingLight" :!class /Script/Engine.PrimitiveComponent))
  (LocalVariables|SetDMI _returnvalue)
  (Rendering|Components|Light|SetCastShadows _spotlight (Variables|Default|GetCastShadows))
  (Rendering|Components|Light|SetIntensity _spotlight _lightintensity)
  (if (Variables|Default|GetLightToggle)
    (Rendering|Material|SetScalarParameterValue (LocalVariables|GetDMI) "None" (/ 0.0 _lightintensity) :!class /Script/Engine.MaterialInstanceDynamic)
    (Rendering|SetVisibility _spotlight true false)
    (else
      (Rendering|Material|SetScalarParameterValue (LocalVariables|GetDMI) "None" 0.0 :!class /Script/Engine.MaterialInstanceDynamic)
      (Rendering|SetVisibility _spotlight false false))))