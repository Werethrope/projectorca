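; Street lighting pole actor for the Industrial City environment, with a toggle that switches its lamp on or off.
; The construction script creates a dynamic instance of the TrafficLight material on the pole mesh and stores it.
; LightToggle drives both that material's StreetLight scalar parameter and the SpotLight's visibility, so the mesh and light stay in sync.
; The event graph holds only disabled placeholder events, so nothing changes the light at runtime.
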(event EventBeginPlay)

(event EventActorBeginOverlap
  (params (OtherActor :type Actor%20Object%20Reference)))

(event EventTick
  (params (DeltaSeconds :type Float%20%28single-precision%29)))

(fn ConstructionScript
  (bind _spotlight (Variables|Default|GetSpotLight))
  (bind _returnvalue (Rendering|Material|CreateDynamicMaterialInstance (Variables|Default|GetStaticMesh) 0 "/Game/IndustrialCity/Materials/-TrafficLight.-TrafficLight" :!class /Script/Engine.PrimitiveComponent))
  (Variables|Default|SetLight_DMI _returnvalue)
  (if (Variables|Default|GetLight%20Toggle)
    (Rendering|Material|SetScalarParameterValue (Variables|Default|GetLight_DMI) "StreetLight" 1.0 :!class /Script/Engine.MaterialInstanceDynamic)
    (Rendering|SetVisibility _spotlight true false)
    (else
      (Rendering|Material|SetScalarParameterValue (Variables|Default|GetLight_DMI) "StreetLight" 0.0 :!class /Script/Engine.MaterialInstanceDynamic)
      (Rendering|SetVisibility _spotlight false false))))